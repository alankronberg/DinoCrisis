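; AI controller for the test carnivore that runs BT_AICarnivore and feeds it perception data for hunting herbivores.
; Perception updates set the herbivore reference and sensed flag on the Blackboard; failed updates clear the flag and write LastKnownLocation, cached from the stimulus's receiver location.
; SetSenseFalse resets sensing after a kill.
; Roam, MoveToAI and Movement form an older AIMoveTo loop that nothing here starts, with roaming now in the tree.
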(event `self.AIPerception.OnTargetPerceptionUpdated`
  (params (Actor :type "Actor Object Reference") (Stimulus :type "AIStimulus Structure"))
  (bind (_age _expirationage _strength _stimuluslocation _receiverlocation _tag _bsuccessfullysensed) (break `AIStimulus` Stimulus))
  (bind _returnvalue (`AIBlueprintHelperLibrary.GetBlackboard` null))
  (bind _returnvalue_2 (`AIBlueprintHelperLibrary.GetBlackboard` null))
  ;[1 1 1] Get a reference to a perceived herbivore for moveto. Also gets last perceived location for move to, should the herbivore escape.
  (if _bsuccessfullysensed
    (bind _asbp_herbivore_character (cast `/Game/Blueprints/DinoAI/AI/TEST_Herbivore/BP_HerbivoreCharacter` Actor)
      (:`then`
        (bind _output_get (set `self.As BP Herbivore Character` _asbp_herbivore_character))
        (`BlackboardComponent.SetValueAsObject` _returnvalue "HerbivoreReference" _output_get)
        (`BlackboardComponent.SetValueAsBool` _returnvalue "CanSenseHerbivore" true)
        (set `self.LastKnownLocation` _receiverlocation))
      (:`CastFailed`
        (`BlackboardComponent.SetValueAsBool` _returnvalue_2 "CanSenseHerbivore" false :!label _label)
        (`BlackboardComponent.SetValueAsVector` _returnvalue_2 "LastKnownLocation" (`self.LastKnownLocation`))
        (set `self.As BP Herbivore Character` null)))
    (else
      (goto _label))))

(event `self.ReceiveBeginPlay`
  (`self.RunBehaviorTree` "/Game/Blueprints/DinoAI/AI/TEST_Carnivore/BT_AICarnivore.BT_AICarnivore")
  (`BlackboardComponent.SetValueAsVector` (`AIBlueprintHelperLibrary.GetBlackboard` null) "ZeroLocation" (0.0 0.0 0.0)))

(event `SetSenseFalse`
  ;[1 1 1] When carnivore eats herbivore, set bb values to false
  (`KismetSystemLibrary.PrintString` "SetSenseFalse")
  (`BlackboardComponent.SetValueAsBool` (`AIBlueprintHelperLibrary.GetBlackboard` null) "CanSenseHerbivore" false)
  (set `self.As BP Herbivore Character` null))

(event `Roam`
  ;[1 1 1] Used for roaming. This is now done in the BT
  (`KismetSystemLibrary.Delay` 0.2)
  (`|AIMoveTo` (`self.K2_GetPawn`) (`NavigationSystemV1.K2_GetRandomReachablePointInRadius` (`self.K2_GetActorLocation`) 1500.0 null null) null
    (:`OnSuccess`
      (`KismetSystemLibrary.PrintString` "MoveTo: True" true true (struct :`G` 0.66 :`B` 1.0 :`A` 1.0) 5.0))
    (:`OnFail`
      (`KismetSystemLibrary.PrintString` "MoveTo: False" true true (struct :`G` 0.66 :`B` 1.0 :`A` 1.0) 5.0)))
  (`self.Movement`))

(event `Move To AI`
  ;[1 1 1] Gets all Herbivore Actors and then selects the 0 index in the array
  ; and gets its location; the Controller moves the Carnivore to that location.
  ; [ONLY WORKS WITH A SINGEL HERBIVORE RIGHT NOW]
  (bind _outactors (`GameplayStatics.GetAllActorsOfClass` "/Game/Blueprints/DinoAI/AI/TEST_Herbivore/BP_HerbivoreCharacter.BP_HerbivoreCharacter_C"))
  (`|AIMoveTo` (`self.K2_GetPawn`) (`self.K2_GetActorLocation` (`|GetArrayItem` _outactors)) null
    (:`OnSuccess`
      (`KismetSystemLibrary.PrintString` "Move To: True"))
    (:`OnFail`
      (`KismetSystemLibrary.PrintString` "Move To: False")))
  (`self.Movement`))

(event `Movement`
  (if true
    (`self.Move To AI`)
    (else
      (`self.Roam`))))

(fn `UserConstructionScript`)