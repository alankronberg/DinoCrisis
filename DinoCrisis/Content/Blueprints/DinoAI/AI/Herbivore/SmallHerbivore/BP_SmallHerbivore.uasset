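; Small herbivore dinosaur character that reacts to being caught by a carnivore.
; When its Box overlaps a BP_BaseCarnivore, it launches itself forward with a slight lift and loses health.
; At zero health it destroys itself and calls SetSenseFalse on that carnivore's AI controller.
; Otherwise it checks its injury status and slows its movement if injured.
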(event `self.Box.OnComponentBeginOverlap`
  (params (OverlappedComponent :type "PrimitiveComponent Object Reference") (OtherActor :type "Actor Object Reference") (OtherComp :type "PrimitiveComponent Object Reference") (OtherBodyIndex :type Integer) (bFromSweep :type Boolean) (SweepResult :type "HitResult Structure (by ref)"))
  (bind _asbp_base_carnivore (cast `/Game/Blueprints/DinoAI/AI/Carnivore/BP_BaseCarnivore` OtherActor))
  (`self.LaunchCharacter` (+ (* (`self.GetActorForwardVector`) 3000) (0.0 0.0 100.0)) true true)
  (`self.DecrementHealth`)
  (if (== (`self.Health`) 0)
    (`self.K2_DestroyActor`)
    (bind _asbp_base_carnivore_aicontroller (cast `/Game/Blueprints/DinoAI/AI/Carnivore/BP_BaseCarnivoreAIController` (`AIBlueprintHelperLibrary.GetAIController` _asbp_base_carnivore)))
    (`/Game/Blueprints/DinoAI/AI/Carnivore/BP_BaseCarnivoreAIController.SetSenseFalse` _asbp_base_carnivore_aicontroller)
    (else
      (`self.CheckInjuryStatus`)
      (if (`self.IsInjured`)
        (`self.SetMovementSpeedSlow`)))))

(fn `UserConstructionScript`
  (`parent.UserConstructionScript`))