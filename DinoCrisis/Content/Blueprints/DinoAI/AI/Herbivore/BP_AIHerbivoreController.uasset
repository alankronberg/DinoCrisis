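; AI controller for herbivore dinosaurs that runs the BT_AIHerbivore behavior tree on BeginPlay.
; AI perception updates feed the blackboard: sensed vegetation sets VegetationReference and CanSenseVegetation, while a lost stimulus clears only the flag.
; SetSenseFalse lets other logic reset that flag and the cached vegetation variable, leaving the blackboard reference intact.
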(event `self.ReceiveBeginPlay`
  (`self.RunBehaviorTree` "/Game/Blueprints/DinoAI/AI/Herbivore/BT_AIHerbivore.BT_AIHerbivore"))

(event `self.AIPerception.OnTargetPerceptionUpdated`
  (params (Actor :type "Actor Object Reference") (Stimulus :type "AIStimulus Structure"))
  (bind _returnvalue (`AIBlueprintHelperLibrary.GetBlackboard` null))
  (if (`.bSuccessfullySensed` (break `AIStimulus` Stimulus))
    (bind _asvegetation (cast `/Game/Blueprints/DinoAI/AI/Herbivore/Vegetation` Actor))
    (bind _output_get (set `self.As Vegetation` _asvegetation))
    (`BlackboardComponent.SetValueAsObject` _returnvalue "VegetationReference" _output_get)
    (`BlackboardComponent.SetValueAsBool` _returnvalue "CanSenseVegetation" true)
    (else
      (`BlackboardComponent.SetValueAsBool` _returnvalue "CanSenseVegetation" false))))

(event `SetSenseFalse`
  ;[1 1 1] When herbivore eats carnivore, set bb values to false
  (`KismetSystemLibrary.PrintString` "SetSenseFalse")
  (`BlackboardComponent.SetValueAsBool` (`AIBlueprintHelperLibrary.GetBlackboard` null) "CanSenseVegetation" false)
  (set `self.As Vegetation` null))

(fn `UserConstructionScript`)