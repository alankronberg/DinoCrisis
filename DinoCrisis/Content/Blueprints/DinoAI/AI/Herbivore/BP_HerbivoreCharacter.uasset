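; Herbivore dinosaur character that manages health through being bitten, eating and gradual decline over time.
; One box overlap with a carnivore removes health, while a second box overlap with vegetation restores it without a cap.
; A looping timer drains health, and both damage paths call a death check that destroys the actor at depleted health.
; A fatal bite also calls SetSenseFalse on the attacking carnivore's AI controller.
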(event `self.Box.OnComponentBeginOverlap`
  (params (OverlappedComponent :type "PrimitiveComponent Object Reference") (OtherActor :type "Actor Object Reference") (OtherComp :type "PrimitiveComponent Object Reference") (OtherBodyIndex :type Integer) (bFromSweep :type Boolean) (SweepResult :type "HitResult Structure (by ref)"))
  (bind _asbp_carnivore_character (cast `/Game/Blueprints/DinoAI/AI/Carnivore/BP_CarnivoreCharacter` OtherActor))
  (set `self.Health` (- (`self.Health`) 200))
  (`KismetSystemLibrary.PrintString` "Ouch! HerbivoreBitten")
  (`KismetSystemLibrary.PrintString` (`KismetStringLibrary.Conv_IntToString` (`self.Health`)))
  (`self.DinosDieWhenTheyAreDead`)
  (if (not (`self.IsAlive`))
    (bind _asbp_aicarnivore_controller (cast `/Game/Blueprints/DinoAI/AI/Carnivore/BP_AICarnivoreController` (`AIBlueprintHelperLibrary.GetAIController` _asbp_carnivore_character)))
    (`/Game/Blueprints/DinoAI/AI/Carnivore/BP_AICarnivoreController.SetSenseFalse` _asbp_aicarnivore_controller)))

(event `self.Box1.OnComponentBeginOverlap`
  (params (OverlappedComponent :type "PrimitiveComponent Object Reference") (OtherActor :type "Actor Object Reference") (OtherComp :type "PrimitiveComponent Object Reference") (OtherBodyIndex :type Integer) (bFromSweep :type Boolean) (SweepResult :type "HitResult Structure (by ref)"))
  (cast `/Game/Blueprints/DinoAI/AI/Herbivore/Vegetation` OtherActor)
  (set `self.Health` (+ (`self.Health`) 200))
  (`KismetSystemLibrary.PrintString` "Found Food!")
  (`KismetSystemLibrary.PrintString` (`KismetStringLibrary.Conv_IntToString` (`self.Health`))))

(event `self.ReceiveBeginPlay`
  (`KismetSystemLibrary.K2_SetTimerDelegate` (delegate `HealthDecrement`) 10.0 true))

(event `HealthDecrement`
  (set `self.Health` (- (`self.Health`) 10))
  (`KismetSystemLibrary.PrintString` "Herbivore Decremented!")
  (`self.DinosDieWhenTheyAreDead`))

(fn `DinosDieWhenTheyAreDead`
  (if (> 1 (`self.Health`))
    (`self.K2_DestroyActor`)
    (set `self.IsAlive` false)))

(fn `UserConstructionScript`)