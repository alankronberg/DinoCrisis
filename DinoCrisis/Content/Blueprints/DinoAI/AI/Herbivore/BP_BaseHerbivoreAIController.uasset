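; AI controller for herbivore dinosaurs that feeds vegetation perception into the Blackboard.
; Perception updates on a BP_BaseHerbivore pawn set IsHungry; sensed BP_Vegetation is stored as VegetationReference, with CanSenseVegetation tracking detection.
; The hunger test is hardcoded true with a debug print, leaving the pawn's Hunger values unused.
; SetSenseFalse clears the sense flag and cached vegetation, but not the Blackboard reference.
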(event `self.AIPerception.OnTargetPerceptionUpdated`
  (params (Actor :type "Actor Object Reference") (Stimulus :type "AIStimulus Structure"))
  (bind _returnvalue (`AIBlueprintHelperLibrary.GetBlackboard` null))
  (bind _returnvalue_2 (`AIBlueprintHelperLibrary.GetBlackboard` null))
  (bind _asbp_base_herbivore (cast `/Game/Blueprints/DinoAI/AI/Herbivore/BP_BaseHerbivore` (`self.K2_GetPawn`)))
  (set `self.IsHungry` (> 1 0))
  (if (`self.IsHungry`)
    (`KismetSystemLibrary.PrintString` "IsHungry")
    (`BlackboardComponent.SetValueAsBool` _returnvalue_2 "IsHungry" true)
    (if (`.bSuccessfullySensed` (break `AIStimulus` Stimulus))
      (bind _asbp_vegetation (cast `/Game/Blueprints/DinoAI/AI/Herbivore/BP_Vegetation` Actor))
      (bind _output_get (set `self.As Vegetation` _asbp_vegetation))
      (`BlackboardComponent.SetValueAsObject` _returnvalue "VegetationReference" _output_get)
      (`BlackboardComponent.SetValueAsBool` _returnvalue "CanSenseVegetation" true)
      (else
        (`BlackboardComponent.SetValueAsBool` _returnvalue "CanSenseVegetation" false)))
    (else
      (`BlackboardComponent.SetValueAsBool` _returnvalue_2 "IsHungry" false))))

(event `SetSenseFalse`
  (`BlackboardComponent.SetValueAsBool` (`AIBlueprintHelperLibrary.GetBlackboard` null) "CanSenseVegetation" false)
  (set `self.As Vegetation` null)
  (set `self.HasVeg` false))

(fn `UserConstructionScript`
  (`parent.UserConstructionScript`))