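; BP_CarnivoreCharacter is a carnivore dinosaur AI character with a simple hunger-style health system.
; A looping timer drains Health at a fixed interval and then runs a death check that destroys the actor once Health runs out.
; Overlapping a BP_HerbivoreCharacter with its Box component restores a large amount of Health, with debug prints tracking both changes.
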(event `self.Box.OnComponentBeginOverlap`
  (params (OverlappedComponent :type "PrimitiveComponent Object Reference") (OtherActor :type "Actor Object Reference") (OtherComp :type "PrimitiveComponent Object Reference") (OtherBodyIndex :type Integer) (bFromSweep :type Boolean) (SweepResult :type "HitResult Structure (by ref)"))
  (cast `/Game/Blueprints/DinoAI/AI/Herbivore/BP_HerbivoreCharacter` OtherActor)
  (set `self.Health` (+ 200 (`self.Health`)))
  (`KismetSystemLibrary.PrintString` "GetBittenBitch")
  (`KismetSystemLibrary.PrintString` (`KismetStringLibrary.Conv_IntToString` (`self.Health`))))

(event `self.ReceiveBeginPlay`
  (`KismetSystemLibrary.K2_SetTimerDelegate` (delegate `HealthDecrement`) 10.0 true))

(event `HealthDecrement`
  (set `self.Health` (- (`self.Health`) 10))
  (`KismetSystemLibrary.PrintString` "Carnivore Decremented!")
  (`KismetSystemLibrary.PrintString` (`KismetStringLibrary.Conv_IntToString` (`self.Health`)))
  (`self.DinosDieWhenTheyAreDead`))

(fn `DinosDieWhenTheyAreDead`
  (if (> 1 (`self.Health`))
    (`self.K2_DestroyActor`)
    (set `self.IsAlive` false)))

(fn `UserConstructionScript`)