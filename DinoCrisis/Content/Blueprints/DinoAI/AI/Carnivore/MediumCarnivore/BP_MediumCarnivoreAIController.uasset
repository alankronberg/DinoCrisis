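; AI controller for medium carnivore dinosaurs that turns perception updates into blackboard data for pursuing herbivores, excluding large ones.
; On BeginPlay it runs a behavior tree and seeds a zero location key.
; A sensed herbivore sets the target reference and sense flag, caching the stimulus receiver location.
; Any other update clears the flag and local reference, publishing that cached location as last known.
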(event `self.AIPerception.OnTargetPerceptionUpdated`
  (params (Actor :type "Actor Object Reference") (Stimulus :type "AIStimulus Structure"))
  (bind (_age _expirationage _strength _stimuluslocation _receiverlocation _tag _bsuccessfullysensed) (break `AIStimulus` Stimulus))
  (bind _returnvalue (`AIBlueprintHelperLibrary.GetBlackboard` null))
  (bind _returnvalue_2 (`AIBlueprintHelperLibrary.GetBlackboard` null))
  ;[1 1 1] Get a reference to a perceived herbivore for moveto. Also gets last perceived location for move to, should the herbivore escape.
  ; Will not moveto Large Herbivores.
  (if _bsuccessfullysensed
    (bind _asbp_base_herbivore (cast `/Game/Blueprints/DinoAI/AI/Herbivore/pdBP_BaseHerbivore` Actor)
      (:`then`
        (cast `/Game/Blueprints/DinoAI/AI/Herbivore/LargeHerbivore/pdBP_LargeHerbivore` _asbp_base_herbivore
          (:`then`
            (`BlackboardComponent.SetValueAsBool` _returnvalue "CanSenseHerbivore" false :!label _label)
            (`BlackboardComponent.SetValueAsVector` _returnvalue "LastKnownLocation" (`self.LastKnownLocation`))
            (set `self.As BP Base Herbivore` null))
          (:`CastFailed`
            (bind _output_get (set `self.As BP Base Herbivore` _asbp_base_herbivore))
            (`BlackboardComponent.SetValueAsObject` _returnvalue_2 "HerbivoreReference" _output_get)
            (`BlackboardComponent.SetValueAsBool` _returnvalue_2 "CanSenseHerbivore" true)
            (set `self.LastKnownLocation` _receiverlocation))))
      (:`CastFailed`
        (goto _label)))
    (else
      (goto _label))))

(event `self.ReceiveBeginPlay`
  (`parent.ReceiveBeginPlay`)
  (`self.RunBehaviorTree` null)
  (`BlackboardComponent.SetValueAsVector` (`AIBlueprintHelperLibrary.GetBlackboard` null) "ZeroLocation" (0.0 0.0 0.0)))

(fn `UserConstructionScript`
  (`parent.UserConstructionScript`))