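; Test herbivore dinosaur character with health and hunger that governs its walk speed.
; A looping timer turns hunger into health, or drains health when starving, slowing the dinosaur when injured or starving.
; One box overlap with a carnivore launches it forward, costs health and slows it; another with vegetation restores hunger.
; Zero health destroys it, clearing the carnivore AI's sense only for attack deaths, not starvation.
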(event `DecrementHealth`
  (set `self.Health` (- (`self.Health`) 1))
  (`KismetSystemLibrary.PrintString` "Herbivore Health Decremented. New Health:")
  (`KismetSystemLibrary.PrintString` (`KismetStringLibrary.Conv_IntToString` (`self.Health`))))

(event `self.Box.OnComponentBeginOverlap`
  (params (OverlappedComponent :type "PrimitiveComponent Object Reference") (OtherActor :type "Actor Object Reference") (OtherComp :type "PrimitiveComponent Object Reference") (OtherBodyIndex :type Integer) (bFromSweep :type Boolean) (SweepResult :type "HitResult Structure (by ref)"))
  (bind _asbp_carnivore_character (cast `/Game/Blueprints/DinoAI/AI/TEST_Carnivore/BP_CarnivoreCharacter` OtherActor))
  (`self.LaunchCharacter` (+ (* (`self.GetActorForwardVector`) 3000) (0.0 0.0 100.0)) true true)
  (`self.DecrementHealth`)
  (if (== (`self.Health`) 0)
    (`self.K2_DestroyActor`)
    (bind _asbp_aicarnivore_controller (cast `/Game/Blueprints/DinoAI/AI/TEST_Carnivore/BP_AICarnivoreController` (`AIBlueprintHelperLibrary.GetAIController` _asbp_carnivore_character)))
    (`/Game/Blueprints/DinoAI/AI/TEST_Carnivore/BP_AICarnivoreController.SetSenseFalse` _asbp_aicarnivore_controller)
    (else
      (`self.CheckInjuryStatus`)
      (if true
        (`self.SetMovementSpeedSlow`)))))

(event `IncrementHealth`
  (if (< (`self.Health`) (`self.MAX_HEALTH`))
    (set `self.Health` (+ (`self.Health`) 1))
    (`KismetSystemLibrary.PrintString` "Health Incremented. Current Health:")
    (`KismetSystemLibrary.PrintString` (`KismetStringLibrary.Conv_IntToString` (`self.Health`)))))

(event `self.Box1.OnComponentBeginOverlap`
  (params (OverlappedComponent :type "PrimitiveComponent Object Reference") (OtherActor :type "Actor Object Reference") (OtherComp :type "PrimitiveComponent Object Reference") (OtherBodyIndex :type Integer) (bFromSweep :type Boolean) (SweepResult :type "HitResult Structure (by ref)"))
  (cast `/Game/Blueprints/DinoAI/AI/Herbivore/BP_Vegetation` OtherActor)
  (`self.IncrementHunger`)
  (`self.CheckStarvingStatus`)
  (if (not (`self.IsStarving`))
    (`self.SetMovementSpeedNormal`)))

(event `self.ReceiveBeginPlay`
  (`KismetSystemLibrary.K2_SetTimerDelegate` (delegate `HungerLostAndConvertedOverTime`) 10.0 true))

(event `DecrementHunger`
  (set `self.Hunger` (- (`self.Hunger`) 1))
  (`KismetSystemLibrary.PrintString` "Hunger Decremented. Current Hunger:")
  (`KismetSystemLibrary.PrintString` (`KismetStringLibrary.Conv_IntToString` (`self.Hunger`))))

(event `HungerLostAndConvertedOverTime`
  (`self.CheckStarvingStatus`)
  (if (`self.IsStarving`)
    (`self.DecrementHealth`)
    (if (== (`self.Health`) 0)
      ;[1 1 1 1 12] This will NOT!!! set carnivore sense to false
      (`self.K2_DestroyActor`)
      (else
        (`self.CheckInjuryStatus`)
        (`self.SetMovementSpeedSlow`)))
    (else
      (`self.DecrementHunger`)
      (`self.IncrementHealth`)
      (`self.CheckInjuryStatus`)
      (if (`self.IsInjured`)
        (`self.SetMovementSpeedSlow`)
        (else
          (`self.SetMovementSpeedNormal`))))))

(event `IncrementHunger`
  (if (< (`self.Hunger`) (`self.MAX_HUNGER`))
    (set `self.Hunger` (+ (`self.Hunger`) 1))
    (`KismetSystemLibrary.PrintString` "Hunger Incremented. Current Hunger:")
    (`KismetSystemLibrary.PrintString` (`KismetStringLibrary.Conv_IntToString` (`self.Hunger`)))))

(event `SetMovementSpeedSlow`
  (set `CharacterMovementComponent.MaxWalkSpeed` (`self.SLOW_SPEED`) (`self.CharacterMovement`)))

(event `SetMovementSpeedNormal`
  (set `CharacterMovementComponent.MaxWalkSpeed` (`self.NORMAL_SPEED`) (`self.CharacterMovement`)))

(event `CheckInjuryStatus`
  (if (> (* 0.3 (`KismetMathLibrary.Conv_IntToDouble` (`self.MAX_HEALTH`))) (`KismetMathLibrary.Conv_IntToDouble` (`self.Health`)))
    (set `self.IsInjured` true)
    (`KismetSystemLibrary.PrintString` "Dinosaur is injured")
    (else
      (set `self.IsInjured` false)
      (`KismetSystemLibrary.PrintString` "Dinosaur is healthy"))))

(event `CheckStarvingStatus`
  (if (== (`self.Hunger`) 0)
    (set `self.IsStarving` true)
    (`KismetSystemLibrary.PrintString` "Dino is starving")
    (else
      (set `self.IsStarving` false)
      (`KismetSystemLibrary.PrintString` "Dino is not starving"))))

(fn `UserConstructionScript`)