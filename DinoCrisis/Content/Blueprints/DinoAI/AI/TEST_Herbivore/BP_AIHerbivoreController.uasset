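; AI controller for a test herbivore dinosaur that starts the BT_AIHerbivore behavior tree on BeginPlay.
; Each perception update sets IsHungry in the blackboard by comparing the pawn's Hunger to MAXHUNGER.
; While hungry, it stores sensed BP_Vegetation as VegetationReference and sets CanSenseVegetation, clearing that flag on lost stimuli.
; SetSenseFalse clears the flag and cached vegetation after eating, but leaves the blackboard reference.
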(event `self.ReceiveBeginPlay`
  (`self.RunBehaviorTree` "/Game/Blueprints/DinoAI/AI/TEST_Herbivore/BT_AIHerbivore.BT_AIHerbivore"))

(event `self.AIPerception.OnTargetPerceptionUpdated`
  (params (Actor :type "Actor Object Reference") (Stimulus :type "AIStimulus Structure"))
  (bind _returnvalue (`AIBlueprintHelperLibrary.GetBlackboard` null))
  (bind _returnvalue_2 (`AIBlueprintHelperLibrary.GetBlackboard` null))
  (bind _asbp_herbivore_character (cast `/Game/Blueprints/DinoAI/AI/TEST_Herbivore/BP_HerbivoreCharacter` (`self.K2_GetPawn`)))
  (set `self.IsHungry` (> (`/Game/Blueprints/DinoAI/AI/TEST_Herbivore/BP_HerbivoreCharacter.MAX_HUNGER` _asbp_herbivore_character) (`/Game/Blueprints/DinoAI/AI/TEST_Herbivore/BP_HerbivoreCharacter.Hunger` _asbp_herbivore_character)))
  (if (`self.IsHungry`)
    (`BlackboardComponent.SetValueAsBool` _returnvalue_2 "IsHungry" true)
    (`KismetSystemLibrary.PrintString` "AI - IsHungry: True")
    (if (`.bSuccessfullySensed` (break `AIStimulus` Stimulus))
      (bind _asbp_vegetation (cast `/Game/Blueprints/DinoAI/AI/Herbivore/BP_Vegetation` Actor))
      (bind _output_get (set `self.As Vegetation` _asbp_vegetation))
      (`BlackboardComponent.SetValueAsObject` _returnvalue "VegetationReference" _output_get)
      (`BlackboardComponent.SetValueAsBool` _returnvalue "CanSenseVegetation" true)
      (else
        (`BlackboardComponent.SetValueAsBool` _returnvalue "CanSenseVegetation" false)))
    (else
      (`BlackboardComponent.SetValueAsBool` _returnvalue_2 "IsHungry" false)
      (`KismetSystemLibrary.PrintString` "Ai - IsHungry: False"))))

(event `SetSenseFalse`
  ;[1 1 1] When herbivore eats vegetation, set bb values to false
  (`KismetSystemLibrary.PrintString` "SetSenseFalse")
  (`BlackboardComponent.SetValueAsBool` (`AIBlueprintHelperLibrary.GetBlackboard` null) "CanSenseVegetation" false)
  (set `self.As Vegetation` null)
  (set `self.HasVeg` false))

(fn `UserConstructionScript`)