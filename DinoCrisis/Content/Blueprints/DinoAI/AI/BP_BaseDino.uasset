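; Base dinosaur character for the DinoAI, providing the health, hunger and movement speed rules of a simple survival loop.
; A looping timer started at BeginPlay drains hunger and regenerates health, or drains health while starving and destroys the actor when it runs out.
; Each tick of that timer updates the injured and starving flags, slowing walk speed when either is set.
; Per its own comment, starvation death does not clear carnivore sense.
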(event `DecrementHealth`
  (set `self.Health` (- (`self.Health`) 1)))

(event `IncrementHealth`
  (if (< (`self.Health`) (`self.MAX_HEALTH`))
    (set `self.Health` (+ (`self.Health`) 1))))

(event `DecrementHunger`
  (set `self.Hunger` (- (`self.Hunger`) 1)))

(event `self.ReceiveBeginPlay`
  (`KismetSystemLibrary.K2_SetTimerDelegate` (delegate `HungerLostAndConvertedOverTime`) 10.0 true))

(event `IncrementHunger`
  (if (< (`self.Hunger`) (`self.MAX_HUNGER`))
    (set `self.Hunger` (+ (`self.Hunger`) 1))))

(event `HungerLostAndConvertedOverTime`
  (`self.CheckStarvingStatus`)
  (if (`self.IsStarving`)
    (`self.DecrementHealth`)
    (if (< (`self.Health`) 1)
      ;[1 1 1 1 12] This will NOT!!! set carnivore sense to false
      (`self.K2_DestroyActor`)
      (else
        (`self.CheckInjuryStatus`)
        (`self.SetMovementSpeedSlow`)))
    (else
      (`self.DecrementHunger`)
      (`self.IncrementHealth`)
      (`self.CheckInjuryStatus`)
      (if (`self.IsInjured`)
        (`self.SetMovementSpeedSlow`)
        (else
          (`self.SetMovementSpeedNormal`))))))

(event `SetMovementSpeedSlow`
  (set `CharacterMovementComponent.MaxWalkSpeed` (`self.SLOW_SPEED`) (`self.CharacterMovement`)))

(event `SetMovementSpeedNormal`
  (set `CharacterMovementComponent.MaxWalkSpeed` (`self.NORMAL_SPEED`) (`self.CharacterMovement`)))

(event `CheckInjuryStatus`
  (if (> (* 0.3 (`KismetMathLibrary.Conv_IntToDouble` (`self.MAX_HEALTH`))) (`KismetMathLibrary.Conv_IntToDouble` (`self.Health`)))
    (set `self.IsInjured` true)
    (else
      (set `self.IsInjured` false))))

(event `CheckStarvingStatus`
  (if (== (`self.Hunger`) 0)
    (set `self.IsStarving` true)
    (else
      (set `self.IsStarving` false))))

(fn `UserConstructionScript`)