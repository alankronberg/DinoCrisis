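; BP_TestPlayer is a test player that places a cursor cube where the camera looks and detects overlaps on mouse clicks.
; Each tick, a Visibility line trace from the camera moves the Cube just above the hit location.
; Holding left or right mouse enables query-only Box collision and sets IncrementValue positive or negative; releasing disables it.
; Box overlaps only print the other actor's name, and IncrementValue is never read here.
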(event `Key|LeftMouseButton`
  (params (Key :type "Key Structure"))
  (bind _box (`self.Box`))
  (:`Pressed`
    (set `self.IncrementValue` 1)
    (`PrimitiveComponent.SetCollisionEnabled` _box "QueryOnly"))
  (:`Released`
    (`PrimitiveComponent.SetCollisionEnabled` _box "NoCollision")))

(event `Key|RightMouseButton`
  (params (Key :type "Key Structure"))
  (bind _box (`self.Box`))
  (:`Pressed`
    (set `self.IncrementValue` -1)
    (`PrimitiveComponent.SetCollisionEnabled` _box "QueryOnly"))
  (:`Released`
    (`PrimitiveComponent.SetCollisionEnabled` _box "NoCollision")))

(event `self.ReceiveTick`
  (params (DeltaSeconds :type "Float (single-precision)"))
  (bind _camera (`self.Camera`))
  (bind _returnvalue (`SceneComponent.K2_GetComponentLocation` _camera))
  (bind _outhit (`KismetSystemLibrary.LineTraceSingle` _returnvalue (+ _returnvalue (* (`KismetMathLibrary.GetForwardVector` (`SceneComponent.K2_GetComponentRotation` _camera)) 1500)) "TraceTypeQuery1"))
  (`SceneComponent.K2_SetWorldLocation` (`self.Cube`) (+ (`.Location` (`GameplayStatics.BreakHitResult` _outhit)) (0.0 0.0 2.0)) false true))

(event `self.Box.OnComponentBeginOverlap`
  (params (OverlappedComponent :type "PrimitiveComponent Object Reference") (OtherActor :type "Actor Object Reference") (OtherComp :type "PrimitiveComponent Object Reference") (OtherBodyIndex :type Integer) (bFromSweep :type Boolean) (SweepResult :type "HitResult Structure (by ref)"))
  (`KismetSystemLibrary.PrintString` (`KismetSystemLibrary.GetDisplayName` OtherActor)))

(fn `UserConstructionScript`)