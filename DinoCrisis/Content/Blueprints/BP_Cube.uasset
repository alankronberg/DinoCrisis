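; BP_Cube is an actor that places eight corner components at the vertices of an axis-aligned cube centred on its location.
; On BeginPlay it halves Height into HalfHeight and calls AdjustCorners, which teleports each corner to a world-space offset of plus or minus HalfHeight on every axis.
; The offsets ignore actor rotation and scale, and the construction script is empty, so this layout is applied only at runtime.
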(event `self.ReceiveBeginPlay`
  (set `self.HalfHeight` (/ (`self.Height`) 2.0))
  (`self.AdjustCorners`))

(fn `AdjustCorners`
  (bind (_returnvalue_x _returnvalue_y _returnvalue_z) (`KismetMathLibrary.BreakVector` (`self.K2_GetActorLocation`)))
  (bind _halfheight (`self.HalfHeight`))
  (bind _returnvalue (- _returnvalue_x _halfheight))
  (bind _returnvalue_2 (- _returnvalue_y _halfheight))
  (bind _returnvalue_3 (- _returnvalue_z _halfheight))
  (bind _returnvalue_4 (+ _returnvalue_x _halfheight))
  (bind _returnvalue_5 (+ _returnvalue_y _halfheight))
  (bind _returnvalue_6 (+ _returnvalue_z _halfheight))
  (`SceneComponent.K2_SetWorldLocation` (`self.Corner0`) (`KismetMathLibrary.MakeVector` _returnvalue _returnvalue_2 _returnvalue_3) false true)
  (`SceneComponent.K2_SetWorldLocation` (`self.Corner1`) (`KismetMathLibrary.MakeVector` _returnvalue_4 _returnvalue_2 _returnvalue_3) false true)
  (`SceneComponent.K2_SetWorldLocation` (`self.Corner2`) (`KismetMathLibrary.MakeVector` _returnvalue_4 _returnvalue_5 _returnvalue_3) false true)
  (`SceneComponent.K2_SetWorldLocation` (`self.Corner3`) (`KismetMathLibrary.MakeVector` _returnvalue _returnvalue_5 _returnvalue_3) false true)
  (`SceneComponent.K2_SetWorldLocation` (`self.Corner4`) (`KismetMathLibrary.MakeVector` _returnvalue _returnvalue_2 _returnvalue_6) false true)
  (`SceneComponent.K2_SetWorldLocation` (`self.Corner5`) (`KismetMathLibrary.MakeVector` _returnvalue_4 _returnvalue_2 _returnvalue_6) false true)
  (`SceneComponent.K2_SetWorldLocation` (`self.Corner6`) (`KismetMathLibrary.MakeVector` _returnvalue_4 _returnvalue_5 _returnvalue_6) false true)
  (`SceneComponent.K2_SetWorldLocation` (`self.Corner7`) (`KismetMathLibrary.MakeVector` _returnvalue _returnvalue_5 _returnvalue_6) false true))

(fn `UserConstructionScript`)