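; VR player pawn for a dinosaur game, with thumbstick movement, a laser pointer and a socket-attached shop menu.
; The right trigger clicks the menu or fires a traced laser with an impact marker.
; PlaceDino traces from the controller to spawn the selected large dinosaur, checking and adjusting GameMode points.
; Increment/decrement inputs toggle a query box with a signed value; debug keys save and load through the pawn and GameMode.
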(event `self.ReceiveBeginPlay`
  (bind _returnvalue (`|CreateWidget` "/Game/Blueprints/UI/VRFPSCounter.VRFPSCounter_C" (`GameplayStatics.GetPlayerController` 0)))
  (`UserWidget.AddToViewport` _returnvalue 0))

(event `InputAction|PlaceDino`
  (params (Key :type "Key Structure"))
  (bind _controllermesh (`self.ControllerMesh`))
  (bind _returnvalue (`SceneComponent.GetSocketLocation` _controllermesh "Laser_Spawn"))
  (:`Pressed`
    (bind _outhit (`KismetSystemLibrary.LineTraceSingle` _returnvalue (+ _returnvalue (* (`KismetMathLibrary.GetForwardVector` (`SceneComponent.GetSocketRotation` _controllermesh "Laser_Spawn")) 1500)) "TraceTypeQuery1"))
    (bind _asbp_dino_game_mode (cast `/Game/Blueprints/BP_DinoGameMode` (`GameplayStatics.GetGameMode`)))
    (bind _output_get (set `self.As BP Dino Game Mode` _asbp_dino_game_mode))
    (bind _output_get_2 (set `/Game/Blueprints/BP_DinoGameMode.Points` (+ 50 (`/Game/Blueprints/BP_DinoGameMode.Points` _output_get)) _output_get))
    (set `self.CurrentPoints` _output_get_2)
    (if (`self.IsBuyingLargeHerbivore`)
      (if (>= (`self.CurrentPoints`) (`self.LargeCost`))
        (bind (_bblockinghit _binitialoverlap _time _distance _location _impactpoint) (`GameplayStatics.BreakHitResult` _outhit))
        (bind _returnvalue_2 (`AIBlueprintHelperLibrary.SpawnAIFromClass` "/Game/Blueprints/DinoAI/AI_C++/Herbivore/LargeHerbivore/C++_LargeHerbivoreCharacter.C++_LargeHerbivoreCharacter_C" null _impactpoint (struct) false null))
        (`/Engine/EditorBlueprintResources/StandardMacros.IsValid` _returnvalue_2
          (:`Is Valid`
            (set `self.IsBuyingLargeHerbivore` false)
            (set `/Game/Blueprints/BP_DinoGameMode.Points` (+ (`/Game/Blueprints/BP_DinoGameMode.Points` (`self.As BP Dino Game Mode`)) 10000) (`self.As BP Dino Game Mode`)))))
      (elif (`self.IsBuyingLargeCarnivore`)
        (if (>= (`self.CurrentPoints`) (`self.LargeCost`))
          (bind _returnvalue_3 (`AIBlueprintHelperLibrary.SpawnAIFromClass` "/Game/Blueprints/DinoAI/AI_C++/Carnivore/LargeCarnivore/C++_LargeCarnivoreCharacter.C++_LargeCarnivoreCharacter_C" null _impactpoint (struct) false null))
          (`/Engine/EditorBlueprintResources/StandardMacros.IsValid` _returnvalue_3
            (:`Is Valid`
              (set `self.IsBuyingLargeCarnivore` false)
              (set `/Game/Blueprints/BP_DinoGameMode.Points` (- (`/Game/Blueprints/BP_DinoGameMode.Points` (`self.As BP Dino Game Mode`)) (`self.LargeCost`)) (`self.As BP Dino Game Mode`)))))))))

(event `InputAction|MotionControllerRightTrigger`
  (params (Key :type "Key Structure"))
  (bind _menushowing (`self.MenuShowing`))
  (:`Pressed`
    (if _menushowing
      (`WidgetInteractionComponent.PressPointerKey` (`self.WidgetInteraction`) "LeftMouseButton")
      (else
        (set `self.IsFiring` true)))
    (`SceneComponent.SetVisibility` (`self.LaserParticle`) true false))
  (:`Released`
    (if _menushowing
      (`WidgetInteractionComponent.ReleasePointerKey` (`self.WidgetInteraction`) "LeftMouseButton")
      (else
        (set `self.IsFiring` false)))
    (`SceneComponent.SetVisibility` (`self.LaserParticle`) false false)))

(event `self.ReceiveTick`
  (params (DeltaSeconds :type "Float (single-precision)"))
  (bind _controllermesh (`self.ControllerMesh`))
  (bind _returnvalue (`SceneComponent.GetSocketLocation` _controllermesh "Laser_Spawn"))
  (if (`self.IsFiring`)
    (bind (_outhit _returnvalue_2) (`KismetSystemLibrary.LineTraceSingle` _returnvalue (+ _returnvalue (* (`KismetMathLibrary.GetForwardVector` (`SceneComponent.GetSocketRotation` _controllermesh "Laser_Spawn")) 1500)) "TraceTypeQuery1"))
    (bind (_bblockinghit _binitialoverlap _time _distance _location _impactpoint _normal _impactnormal _physmat _hitactor _hitcomponent _hitbonename _hititem _faceindex _tracestart _traceend) (`GameplayStatics.BreakHitResult` _outhit))
    (`ParticleSystemComponent.SetBeamSourcePoint` (`self.LaserParticle`) 0 _tracestart 0)
    (if _returnvalue_2
      (`SceneComponent.K2_SetWorldLocationAndRotation` (`self.Sphere`) _impactpoint (`KismetMathLibrary.MakeRotFromYX` _normal (`KismetMathLibrary.Conv_RotatorToVector` (`SceneComponent.K2_GetComponentRotation` (`self.Sphere`)))) false false)
      (`SceneComponent.SetVisibility` (`self.Sphere`) true false)
      (`ParticleSystemComponent.SetBeamTargetPoint` (`self.LaserParticle`) 0 _impactpoint 0)
      (else
        (`ParticleSystemComponent.SetBeamTargetPoint` (`self.LaserParticle`) 0 _traceend 0)
        (`SceneComponent.SetVisibility` (`self.Sphere`) false false :!label _label)))
    (else
      (goto _label))))

(event `InputAxis|InputAxisX`
  (params (AxisValue :type "Float (single-precision)"))
  (`self.AddControllerPitchInput` AxisValue))

(event `Key|LeftMouseButton`
  (params (Key :type "Key Structure"))
  (bind _box (`self.Box`))
  (:`Pressed`
    (set `self.incrementValue` 1 :!label _label_2)
    (`PrimitiveComponent.SetCollisionEnabled` _box "QueryOnly"))
  (:`Released`
    (`PrimitiveComponent.SetCollisionEnabled` _box "NoCollision" :!label _label_3)))

(event `InputAxis|MotionControllerThumbLeft_X`
  (params (AxisValue :type "Float (single-precision)"))
  (`self.AddMovementInput` (* (`KismetMathLibrary.ProjectVectorOnToPlane` (`SceneComponent.GetRightVector` (`self.Camera`))) AxisValue) (`self.MovementSpeed`)))

(event `Key|One`
  (params (Key :type "Key Structure"))
  ;[1 1 1] Game Saving
  (:`Pressed`
    (`self.SaveGame`)
    (bind _asbp_dino_game_mode (cast `/Game/Blueprints/BP_DinoGameMode` (`GameplayStatics.GetGameMode`)))
    (`/Game/Blueprints/BP_DinoGameMode.SaveGame` _asbp_dino_game_mode)
    (`/Game/Blueprints/BP_DinoGameMode.SaveDinos` _asbp_dino_game_mode null)
    (`/Game/Blueprints/BP_DinoGameMode.SaveVegetation` _asbp_dino_game_mode null)
    (`/Game/Blueprints/BP_DinoGameMode.SavePoints` _asbp_dino_game_mode null)))

(event `InputAction|Increment`
  (params (Key :type "Key Structure"))
  (:`Pressed`
    (goto _label_2))
  (:`Released`
    (goto _label_3)))

(event `Key|RightMouseButton`
  (params (Key :type "Key Structure"))
  (bind _box (`self.Box`))
  (:`Pressed`
    (set `self.IncrementValue` -1 :!label _label_4)
    (`PrimitiveComponent.SetCollisionEnabled` _box "QueryOnly"))
  (:`Released`
    (`PrimitiveComponent.SetCollisionEnabled` _box "NoCollision" :!label _label_5)))

(event `InputAxis|MotionControllerThumbLeft_Y`
  (params (AxisValue :type "Float (single-precision)"))
  (`self.AddMovementInput` (* (`KismetMathLibrary.ProjectVectorOnToPlane` (`SceneComponent.GetForwardVector` (`self.Camera`))) AxisValue) (`self.MovementSpeed`)))

(event `InputAction|Decrement`
  (params (Key :type "Key Structure"))
  (:`Pressed`
    (goto _label_4))
  (:`Released`
    (goto _label_5)))

(event `Key|Two`
  (params (Key :type "Key Structure"))
  ;[1 1 1] Game Loading
  (:`Pressed`
    (`self.LoadGame`)
    (bind _asbp_dino_game_mode (cast `/Game/Blueprints/BP_DinoGameMode` (`GameplayStatics.GetGameMode`)))
    (`/Game/Blueprints/BP_DinoGameMode.LoadGame` _asbp_dino_game_mode)
    (`/Game/Blueprints/BP_DinoGameMode.LoadDinos` _asbp_dino_game_mode null)
    (`/Game/Blueprints/BP_DinoGameMode.LoadVegetation` _asbp_dino_game_mode null)
    (`/Game/Blueprints/BP_DinoGameMode.LoadPoints` _asbp_dino_game_mode null)))

(event `InputAction|ShowMenu`
  (params (Key :type "Key Structure")))

(event `InputAction|ShowMenu`
  (params (Key :type "Key Structure"))
  (:`Pressed`
    (if (`self.MenuShowing`)
      (`self.K2_DestroyActor` (`self.ShopMenuWidget`))
      (`ActorComponent.Deactivate` (`self.WidgetInteraction`))
      (set `self.MenuShowing` false)
      (else
        (bind _returnvalue (`|SpawnActorFromClass` "/Game/Blueprints/UI/PlayingMenus/BP_GameMenuWidgetActor.BP_GameMenuWidgetActor_C" (`SceneComponent.GetSocketTransform` (`self.SkeletalMesh`) "MenuSocket" "RTS_ParentBoneSpace") "Undefined" "OverrideRootScale" null null))
        (bind _output_get (set `self.ShopMenuWidget` _returnvalue))
        (`self.K2_AttachToComponent` _output_get (`self.SkeletalMesh`) "MenuSocket" "KeepRelative" "KeepRelative" "KeepRelative" true)
        (`ActorComponent.Activate` (`self.WidgetInteraction`) false)
        (set `self.MenuShowing` true)))))

(fn `NewFunction_0`
  (params (self2 :type "SceneComponent Object Reference"))
  (`SceneComponent.SetVisibility` self2 false false))

(fn `UserConstructionScript`)