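; VR player pawn for world creation, with thumbstick movement, a laser pointer and a toggleable hand-socket menu.
; While the trigger is held, a line trace drives the beam and surface-aligned sphere cursor, or clicks widgets when the menu is open.
; Increment/Decrement inputs set a signed step and briefly enable Box query collision.
; Keys 5/6 save and load through BP_DinoGameMode; older save attempts remain as unconnected nodes.
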(event `self.ReceiveBeginPlay`
  (set `self.incrementActor` (`self.Cube`))
  (set `self.decrementActor` (`self.Cube1`))
  (bind _returnvalue (`|CreateWidget` "/Game/Blueprints/UI/VRFPSCounter.VRFPSCounter_C" (`GameplayStatics.GetPlayerController` 0)))
  (`UserWidget.AddToViewport` _returnvalue 0))

(event `InputAction|MotionControllerRightTrigger`
  (params (Key :type "Key Structure"))
  (bind _menushowing (`self.MenuShowing`))
  (:`Pressed`
    (if _menushowing
      (`WidgetInteractionComponent.PressPointerKey` (`self.WidgetInteraction`) "LeftMouseButton")
      (else
        (set `self.IsFiring` true)))
    (`SceneComponent.SetVisibility` (`self.LaserParticle`) true false))
  (:`Released`
    (if _menushowing
      (`WidgetInteractionComponent.ReleasePointerKey` (`self.WidgetInteraction`) "LeftMouseButton")
      (else
        (set `self.IsFiring` false)))
    (`SceneComponent.SetVisibility` (`self.LaserParticle`) false false)))

(event `self.ReceiveTick`
  (params (DeltaSeconds :type "Float (single-precision)"))
  (bind _controllermesh (`self.ControllerMesh`))
  (bind _returnvalue (`SceneComponent.GetSocketLocation` _controllermesh "Laser_Spawn"))
  (if (`self.IsFiring`)
    (if (not (`self.MenuShowing`))
      (bind (_outhit _returnvalue_2) (`KismetSystemLibrary.LineTraceSingle` _returnvalue (+ _returnvalue (* (`KismetMathLibrary.GetForwardVector` (`SceneComponent.GetSocketRotation` _controllermesh "Laser_Spawn")) 1500)) "TraceTypeQuery1"))
      (bind (_bblockinghit _binitialoverlap _time _distance _location _impactpoint _normal _impactnormal _physmat _hitactor _hitcomponent _hitbonename _hititem _faceindex _tracestart _traceend) (`GameplayStatics.BreakHitResult` _outhit))
      (`ParticleSystemComponent.SetBeamSourcePoint` (`self.LaserParticle`) 0 _tracestart 0)
      (if _returnvalue_2
        (`SceneComponent.K2_SetWorldLocationAndRotation` (`self.Sphere`) _impactpoint (`KismetMathLibrary.MakeRotFromYX` _normal (`KismetMathLibrary.Conv_RotatorToVector` (`SceneComponent.K2_GetComponentRotation` (`self.Sphere`)))) false false)
        (`SceneComponent.SetVisibility` (`self.Sphere`) true false)
        (`ParticleSystemComponent.SetBeamTargetPoint` (`self.LaserParticle`) 0 _impactpoint 0)
        (else
          (`ParticleSystemComponent.SetBeamTargetPoint` (`self.LaserParticle`) 0 _traceend 0)
          (`SceneComponent.SetVisibility` (`self.Sphere`) false false :!label _label))))
    (else
      (goto _label))))

(event `InputAxis|InputAxisX`
  (params (AxisValue :type "Float (single-precision)"))
  (`self.AddControllerPitchInput` AxisValue))

(event `InputAxis|MotionControllerThumbLeft_X`
  (params (AxisValue :type "Float (single-precision)"))
  (`self.AddMovementInput` (* (`KismetMathLibrary.ProjectVectorOnToPlane` (`SceneComponent.GetRightVector` (`self.Camera`))) AxisValue) (`self.MovementSpeed`)))

(event `InputAction|Increment`
  (params (Key :type "Key Structure"))
  (bind _box (`self.Box`))
  (:`Pressed`
    (if (`SceneComponent.IsVisible` (`self.Sphere`))
      _
      (else
        _))
    (set `self.incrementValue` 1)
    (`PrimitiveComponent.SetCollisionEnabled` _box "QueryOnly"))
  (:`Released`
    (`PrimitiveComponent.SetCollisionEnabled` _box "NoCollision")))

(event `InputAxis|MotionControllerThumbLeft_Y`
  (params (AxisValue :type "Float (single-precision)"))
  (`self.AddMovementInput` (* (`KismetMathLibrary.ProjectVectorOnToPlane` (`SceneComponent.GetForwardVector` (`self.Camera`))) AxisValue) (`self.MovementSpeed`)))

(event `InputAction|Decrement`
  (params (Key :type "Key Structure"))
  (bind _box (`self.Box`))
  (:`Pressed`
    (if (`SceneComponent.IsVisible` (`self.Sphere`))
      _
      (else
        _))
    (set `self.IncrementValue` -1)
    (`PrimitiveComponent.SetCollisionEnabled` _box "QueryOnly"))
  (:`Released`
    (`PrimitiveComponent.SetCollisionEnabled` _box "NoCollision")))

(event `InputAction|ShowMenu`
  (params (Key :type "Key Structure"))
  (:`Pressed`
    (if (`self.MenuShowing`)
      (`self.K2_DestroyActor` (`self.MenuWidget`))
      (`ActorComponent.Deactivate` (`self.WidgetInteraction`))
      (set `self.MenuShowing` false)
      (else
        (bind _returnvalue (`|SpawnActorFromClass` "/Game/Blueprints/BP_WidgetActor.BP_WidgetActor_C" (`SceneComponent.GetSocketTransform` (`self.SkeletalMesh`) "MenuSocket" "RTS_ParentBoneSpace") "Undefined" "OverrideRootScale" null null))
        (bind _output_get (set `self.MenuWidget` _returnvalue))
        (`self.K2_AttachToComponent` _output_get (`self.SkeletalMesh`) "MenuSocket" "KeepRelative" "KeepRelative" "KeepRelative" true)
        (`ActorComponent.Activate` (`self.WidgetInteraction`) false)
        (set `self.MenuShowing` true)))))

(event `Key|Five`
  (params (Key :type "Key Structure"))
  (:`Pressed`
    (bind _asbp_dino_game_mode (cast `/Game/Blueprints/BP_DinoGameMode` (`GameplayStatics.GetGameMode`)))
    (`/Game/Blueprints/BP_DinoGameMode.SaveGame` _asbp_dino_game_mode)))

(event `Key|Six`
  (params (Key :type "Key Structure"))
  (:`Pressed`
    (bind _asbp_dino_game_mode (cast `/Game/Blueprints/BP_DinoGameMode` (`GameplayStatics.GetGameMode`)))
    (`/Game/Blueprints/BP_DinoGameMode.LoadGame` _asbp_dino_game_mode)))

(fn `NewFunction_0`
  (params (self2 :type "SceneComponent Object Reference"))
  (`SceneComponent.SetVisibility` self2 false false))

(fn `UserConstructionScript`)