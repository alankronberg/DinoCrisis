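; VR main menu pawn that lets the player operate widgets with motion controllers.
; On begin play or possession it selects and activates the right widget interaction component.
; The right trigger sends left-mouse presses and releases through that component, while each thumbstick's Y axis scrolls its own hand's component.
; Unconnected leftovers hold failed save/load experiments and left/right hand-switching logic that never runs.
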(event `self.ReceiveBeginPlay`
  (bind _rightwidgetinteraction (`self.RightWidgetInteraction`))
  (set `self.SelectedInteractionWidget` _rightwidgetinteraction :!label _label)
  (`ActorComponent.Activate` _rightwidgetinteraction false))

(event `InputAction|MotionControllerRightTrigger`
  (params (Key :type "Key Structure"))
  (:`Pressed`
    (`WidgetInteractionComponent.PressPointerKey` (`self.RightWidgetInteraction`) "LeftMouseButton"))
  (:`Released`
    (`WidgetInteractionComponent.ReleasePointerKey` (`self.RightWidgetInteraction`) "LeftMouseButton")))

(event `self.ReceivePossessed`
  (params (NewController :type "Controller Object Reference"))
  (goto _label))

(event `self.ReceiveTick`
  (params (DeltaSeconds :type "Float (single-precision)")))

(event `InputAxis|MotionControllerThumbLeft_Y`
  (params (AxisValue :type "Float (single-precision)"))
  (`WidgetInteractionComponent.ScrollWheel` (`self.LeftWidgetInteraction`) AxisValue))

(event `InputAxis|MotionControllerThumbRight_Y`
  (params (AxisValue :type "Float (single-precision)"))
  (`WidgetInteractionComponent.ScrollWheel` (`self.RightWidgetInteraction`) AxisValue))

(fn `NewFunction_0`
  (params (self2 :type "SceneComponent Object Reference"))
  (`SceneComponent.SetVisibility` self2 false false))

(fn `UserConstructionScript`)