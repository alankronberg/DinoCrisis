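; Game mode that saves and loads voxel chunk terrain through two separate routes.
; In the CubeWorld level, a text route has the first chunk overwrite and the rest write, then parses semicolon-separated chunks of comma-separated cubes on load.
; A SaveGame route stores each chunk's dumped data in a BP_SaveTest slot.
; Both loaders match data to chunks by GetAllActorsOfClass order, relying on it staying consistent.
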(event `self.ReceiveBeginPlay`)

(event `SaveMap`
  (bind _returnvalue (`GameplayStatics.GetCurrentLevelName` true))
  (if (`KismetStringLibrary.EqualEqual_StrStr` _returnvalue "CubeWorld")
    (bind _outactors (`GameplayStatics.GetAllActorsOfClass` "/Game/Blueprints/BP_VoxelChunk.BP_VoxelChunk_C"))
    (bind _output_get (set `self.Chunks` _outactors))
    (for (_array_element _array_index) _output_get
      (if (== _array_index 0)
        (`VoxelChunk.Overwrite` _array_element)
        (else
          (`VoxelChunk.WriteTest` _array_element))))))

(event `LoadMapFromFile`
  (bind _returnvalue (`GameplayStatics.GetCurrentLevelName` true))
  (if (`KismetStringLibrary.EqualEqual_StrStr` _returnvalue "CubeWorld")
    (bind _outactors (`GameplayStatics.GetAllActorsOfClass` "/Game/Blueprints/BP_VoxelChunk.BP_VoxelChunk_C"))
    (set `self.Chunks` _outactors)
    (bind _returnvalue_2 (`self.getMapDataFromFile`))
    (set `self.MapData` (`KismetStringLibrary.ParseIntoArray` _returnvalue_2 ";"))
    (for (_array_element _array_index) (`self.Chunks`)
      (`VoxelChunk.InitCubesFromFile` _array_element (`KismetStringLibrary.ParseIntoArray` (`|GetArrayItem` (`self.MapData`) _array_index) ",")))
    (set `self.bLoadMapFromFile` false)))

(event `SaveGame`
  (bind _returnvalue (`GameplayStatics.CreateSaveGameObject` "/Game/Blueprints/BP_SaveTest.BP_SaveTest_C"))
  (bind _outactors (`GameplayStatics.GetAllActorsOfClass` "/Game/Blueprints/BP_VoxelChunk.BP_VoxelChunk_C"))
  (for _array_element _outactors
    (bind _returnvalue_2 (`VoxelChunk.dumpChunkData` _array_element))
    (`KismetArrayLibrary.Array_Add` (`SaveGameObject.Chunks` _returnvalue) (make `ChunkSave` _returnvalue_2)))
  (`GameplayStatics.SaveGameToSlot` _returnvalue "Alan"))

(event `LoadGame`
  (bind _returnvalue (`GameplayStatics.DoesSaveGameExist` "Alan"))
  (if _returnvalue
    (bind _returnvalue_2 (`GameplayStatics.LoadGameFromSlot` "Alan"))
    (bind _asbp_save_test (cast `/Game/Blueprints/BP_SaveTest` _returnvalue_2))
    (bind _outactors (`GameplayStatics.GetAllActorsOfClass` "/Game/Blueprints/BP_VoxelChunk.BP_VoxelChunk_C"))
    (for (_array_element _array_index) _outactors
      (`VoxelChunk.fillChunkData` _array_element (`.data` (break `ChunkSave` (`|GetArrayItem` (`SaveGameObject.Chunks` _asbp_save_test) _array_index)))))))

(fn `UserConstructionScript`)